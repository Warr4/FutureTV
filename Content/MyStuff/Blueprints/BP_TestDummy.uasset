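; BP_TestDummy is a damageable target dummy that respawns itself when killed.
; On BeginPlay it stores its root transform, then stays hidden for two seconds before reappearing.
; AnyDamage subtracts from HP, and at zero or below the dummy spawns a fresh copy at the stored transform and destroys itself, so each replacement repeats the hidden delay.
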(event Collision|EventActorBeginOverlap
  (params (OtherActor :type Actor%20Object%20Reference)))

(event EventTick
  (params (DeltaSeconds :type Float%20%28single-precision%29)))

(event Game|Damage|EventAnyDamage
  (params (Damage :type Float%20%28single-precision%29) (DamageType :type Damage%20Type%20Object%20Reference) (InstigatedBy :type Controller%20Object%20Reference) (DamageCauser :type Actor%20Object%20Reference))
  (bind _output_get (Variables|Default|SetHP (- (Variables|Default|GetHP) Damage)))
  (if (<= _output_get 0.0)
    (Game|SpawnActorfromClass "BP_TestDummy_C" (Variables|Default|GetSpawnLoc) "AlwaysSpawn" "MultiplyWithRoot" 0 0)
    (Actor|DestroyActor)))

(event EventBeginPlay
  (Variables|Default|SetSpawnLoc (Transformation|GetWorldTransform (Variables|Default|GetDefaultSceneRoot)))
  (Rendering|SetActorHiddenInGame true)
  (Utilities|FlowControl|Delay 2.0)
  (Rendering|SetActorHiddenInGame false))

(fn ConstructionScript)