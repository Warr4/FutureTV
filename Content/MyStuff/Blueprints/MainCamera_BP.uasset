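; MainCamera_BP is a camera actor that serves as the player's main view and follows the controlled pawn.
; On BeginPlay it makes itself the view target of player controller 0.
; Every Tick it moves to the pawn's location, raised along Z by a Height variable, without smoothing.
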(event EventBeginPlay
  (bind _returnvalue (Game|GetPlayerController 0))
  (Utilities|IsValid _returnvalue
    (:Is%20Valid
      (Game|Player|SetViewTargetwithBlend _returnvalue self 0.0 "VTBlend_Linear" 0.0 false))))

(event EventTick
  (params (DeltaSeconds :type Float%20%28single-precision%29))
  (bind _returnvalue (Game|GetPlayerController 0))
  (bind _returnvalue_2 (Pawn|GetControlledPawn _returnvalue))
  (bind _returnvalue_3 (Transformation|GetActorLocation _returnvalue_2))
  (Utilities|IsValid _returnvalue_2
    (:Is%20Valid
      (Transformation|SetActorLocation (Math|Vector|MakeVector (.x _returnvalue_3) (.y _returnvalue_3) (+ (.z _returnvalue_3) (Variables|Default|GetHeight))) false false))))

(fn ConstructionScript)