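; AI controller for a melee bot that chases the player and punches on arrival.
; On BeginPlay it gets the bot and its arrow component from the pawn, then starts a looping move-to timer if player pawn 0 is tagged Player.
; A DoOnce gates each punch: turn, delay, debug-drawn line trace from the arrow, damage tagged hits, delay, reset.
; Random wander and FIRE logic exists, but its timer is disconnected.
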(event Custom|Random%20move
  (if (not (Variables|Default|GetSeenPlayer))
    (bind _randomlocation (Class|NavigationSystemV1|GetRandomLocationinNavigableRadius (Transformation|GetActorLocation (Pawn|GetControlledPawn)) 1e+03 0 0))
    (AI|AIMoveTo 0 _randomlocation 0 5.0 false
      (:OnSuccess
        (CallFunction|FIRE)))))

(event Custom|Open%20Do%20Once
  (Utilities|FlowControl|DoOnce false) ; enters at Reset
)

(event Custom|Punch
  (bind _arrow_ref (Variables|Default|GetArrow%20Ref))
  (bind _character_ref (Variables|Default|GetCharacter%20Ref))
  (bind _returnvalue (Transformation|GetWorldTransform _arrow_ref))
  (Transformation|SetActorRotation _character_ref (Math|Rotator|MakeRotator 0.0 0.0 (.yaw (Math|Rotator|FindLookatRotation (Transformation|GetActorLocation _character_ref) (Transformation|GetActorLocation (Variables|Default|GetPlayer))))))
  (Utilities|FlowControl|Delay 0.5)
  (bind _outhit (Collision|LineTraceByChannel (.location _returnvalue) (+ (.location _returnvalue) (* (Math|Rotator|GetRotationXVector (.rotation _returnvalue)) (Variables|Default|GetMeleeRange))) "TraceTypeQuery1" false 0 "ForDuration" true "(R=1.000000,G=0.000000,B=0.000000,A=1.000000)" "(R=0.000000,G=1.000000,B=0.000000,A=1.000000)" 1.0))
  (Utilities|IsValid (.HitActor (Collision|BreakHitResult _outhit))
    (:Is%20Valid
      (if (Actor|ActorHasTag (.HitActor (Collision|BreakHitResult _outhit)) (Variables|Default|GetNPCDamageable))
        (Game|Damage|ApplyDamage (.HitActor (Collision|BreakHitResult _outhit)) 1e+02 0 0)))
    (:Is%20Not%20Valid
      _))
  (Utilities|FlowControl|Delay 0.5)
  (CallFunction|OpenDoOnce))

(event Custom|Chase%20Player
  (bind _returnvalue (Utilities|Time|SetTimerbyEvent (delegate Custom|Move%20to%20player) 0.1 true true))
  (Variables|Default|SetMove%20timer _returnvalue))

(event Custom|Move%20to%20player
  (AI|AIMoveTo (Variables|Default|GetCharacter%20Ref) (Transformation|GetActorLocation (Variables|Default|GetPlayer)) 0 4e+01 true
    (:OnSuccess
      (if (Utilities|IsValid (Variables|Default|GetCharacter%20Ref))
        (Utilities|FlowControl|DoOnce false
          (:Completed
            (CallFunction|Punch)
            (CallFunction|MovetoPlayer)))))))

(event Custom|FIRE
  (if (Variables|Default|GetCanShoot)
    (Transformation|SetActorRotation 0 (Math|Rotator|FindLookatRotation (Transformation|GetActorLocation) (Transformation|GetActorLocation (Variables|Default|GetPlayer))))))

(event EventBeginPlay
  (bind _returnvalue (Game|Player|GetPlayerPawn 0))
  (bind _returnvalue_2 (Pawn|GetControlledPawn))
  (Utilities|FlowControl|Delay 0.1)
  (bind _characterref (Class|BPIGetControlledBot|GetControlledBotActor(Message) _returnvalue_2))
  (Variables|Default|SetCharacter%20Ref _characterref)
  (bind _arrowref (Class|BPIGetControlledBot|GetControlledBotArrowComponent(Message) _returnvalue_2))
  (Variables|Default|SetArrow%20Ref _arrowref)
  (if (Actor|ActorHasTag _returnvalue "Player")
    (Variables|Default|SetPlayer _returnvalue)
    (CallFunction|ChasePlayer)))

(event EventTick
  (params (DeltaSeconds :type Float%20%28single-precision%29)))

(fn ConstructionScript)