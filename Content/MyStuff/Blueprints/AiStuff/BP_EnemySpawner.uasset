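; Enemy spawner Blueprint that spawns a set Amount of SpawningClass actors at its own transform, one at a time.
; Its Spawn event waits briefly, decrements Amount, spawns with collision adjustment, then calls itself until Amount reaches zero or below.
; The count is checked only after spawning, so each call to Spawn produces at least one actor.
; Nothing in this Blueprint starts the Spawn chain.
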(event Custom|Spawn
  (Utilities|FlowControl|Delay 0.1)
  (Variables|Default|SetAmount (+ (Variables|Default|GetAmount) -1))
  (Game|SpawnActorfromClass (Variables|Default|GetSpawningClass) (Transformation|GetActorTransform) "AdjustIfPossibleButAlwaysSpawn" "MultiplyWithRoot" 0 0)
  (if (not (<= (Variables|Default|GetAmount) 0))
    (CallFunction|Spawn)))

(event Collision|EventActorBeginOverlap
  (params (OtherActor :type Actor%20Object%20Reference)))

(fn ConstructionScript)