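; BP_BotTest is a test bot actor that loses HP from any damage and destroys itself at zero.
; Leftover input logic, kept for possible future use, runs a looping FIRE timer while Shoot is held.
; FIRE draws a debug line trace along Arrow1 and damages hit actors tagged as player-damageable.
; Getters expose the bot and its arrow component, while GetEnemyActorClass returns no value.
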(event Custom|FIRE
  (bind _arrow1 (Variables|Default|GetArrow1))
  (bind _returnvalue (Transformation|GetWorldTransform _arrow1))
  ;[1 1 1] Leftover Shoot Logic For Potentual Futeure Use
  (bind _outhit (Collision|LineTraceByChannel (.location _returnvalue) (+ (.location _returnvalue) (* (Math|Rotator|GetRotationXVector (.rotation _returnvalue)) (Variables|Default|GetShoot%20distance))) "TraceTypeQuery1" false 0 "ForDuration" true "(R=1.000000,G=0.000000,B=0.000000,A=1.000000)" "(R=0.000000,G=1.000000,B=0.000000,A=1.000000)" 1.0))
  (Utilities|IsValid (.HitActor (Collision|BreakHitResult _outhit))
    (:Is%20Valid
      (if (Actor|ActorHasTag (.HitActor (Collision|BreakHitResult _outhit)) (Variables|Default|GetPlayerDamageable))
        (Game|Damage|ApplyDamage (.HitActor (Collision|BreakHitResult _outhit)) 1e+01 0 0)))))

(event Game|Damage|EventAnyDamage
  (params (Damage :type Float%20%28single-precision%29) (DamageType :type Damage%20Type%20Object%20Reference) (InstigatedBy :type Controller%20Object%20Reference) (DamageCauser :type Actor%20Object%20Reference))
  ;[1 1 1] Health
  (bind _output_get (Variables|Default|SetHP (- (Variables|Default|GetHP) Damage)))
  (if (<= _output_get 0.0)
    (Actor|DestroyActor)))

(event Input|ActionEvents|InputActionShoot
  (params (Key :type Key%20Structure :default "None"))
  ;[1 1 1] Leftover Shoot Logic For Potentual Futeure Use
  (:Pressed
    (Utilities|Time|SetTimerbyFunctionName 0 "FIRE" (Variables|Default|Getfirerate) true))
  (:Released
    (Utilities|Time|ClearTimerbyFunctionName 0 "FIRE")))

(fn ConstructionScript)

(fn GetControlledBotActor
  (return self))

(fn GetControlledBotArrowComponent
  (return (Variables|Default|GetArrow1)))

(fn GetEnemyActorClass
  (return 0))