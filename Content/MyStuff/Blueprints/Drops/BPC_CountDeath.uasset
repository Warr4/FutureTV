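; Actor component that tallies NPC deaths by counting the destruction of the actor it is attached to.
; On BeginPlay it binds to the owner's OnDestroyed delegate and caches the game instance as GI_CustomGameInstance.
; The CountDeath handler increments KilledNPCs on that game instance, with no check on why the owner was destroyed.
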(event Custom|CountDeath
  (params (DestroyedActor :type Actor%20Object%20Reference))
  (bind _game_instance (Variables|Default|GetGame%20Instance))
  (Variables|/Game/MyStuff/Blueprints/GI_CustomGameInstance.GI_CustomGameInstance_C|SetKilled%20NPCs _game_instance (+ (Variables|/Game/MyStuff/Blueprints/GI_CustomGameInstance.GI_CustomGameInstance_C|GetKilled%20NPCs _game_instance) 1)))

(event EventBeginPlay
  (Game|BindEventtoOnDestroyed (Components|GetOwner) (EventDispatchers|CreateEvent :!event Custom|CountDeath))
  (bind _asgi_custom_game_instance (Utilities|Casting|CastToGI_CustomGameInstance (Game|GetGameInstance)))
  (Variables|Default|SetGame%20Instance _asgi_custom_game_instance))

(event EventTick
  (params (DeltaSeconds :type Float%20%28single-precision%29)))