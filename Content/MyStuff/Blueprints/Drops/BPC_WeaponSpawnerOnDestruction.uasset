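; Actor component that spawns random weapon drops when its owning actor is destroyed.
; On BeginPlay it binds to the owner's OnDestroyed event and caches the custom game instance.
; Unless the game instance flags a respawn, each of the configured item rolls has a roughly 5% chance to spawn a random Drops class at the owner's transform.
; Failed rolls only print a debug string.
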(event Custom|SpawnStuff
  (params (DestroyedActor :type Actor%20Object%20Reference))
  (if (not (Variables|/Game/MyStuff/Blueprints/GI_CustomGameInstance.GI_CustomGameInstance_C|GetIsRespawning (Variables|Default|GetGame%20Instance)))
    (for _index (range 0 (- (Variables|Default|GetNumberOfItemsToSpawn) 1))
      (if (>= (Math|Random|RandomFloatinRange 0.0 1e+02) 95.0)
        (Variables|Default|SetSpawnableVar (Math|Random|RandomInteger (Utilities|Array|Length (Variables|Default|GetDrops))))
        (Game|SpawnActorfromClass (Utilities|Array|Get(acopy) (Variables|Default|GetDrops) (Variables|Default|GetSpawnableVar)) (Transformation|GetActorTransform (Components|GetOwner)) "Undefined" "MultiplyWithRoot" 0 0)
        (else
          (Development|PrintString "SpawnNothing"))))))

(event EventBeginPlay
  (Game|BindEventtoOnDestroyed (Components|GetOwner) (EventDispatchers|CreateEvent :!event Custom|SpawnStuff))
  (bind _asgi_custom_game_instance (Utilities|Casting|CastToGI_CustomGameInstance (Game|GetGameInstance)))
  (Variables|Default|SetGame%20Instance _asgi_custom_game_instance))

(event EventTick
  (params (DeltaSeconds :type Float%20%28single-precision%29)))