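; Base pickup actor for drops that add to the player's score.
; On spawn it applies a small random horizontal force to its mesh, then switches off physics simulation after a short delay.
; OnPickUp checks for the Player tag, adds the given value to Score in GI_CustomGameInstance and destroys the pickup.
; The sphere overlap event is empty, and nothing in this Blueprint calls OnPickUp.
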(event OnComponentBeginOverlap(Sphere)
  (params (OverlappedComponent :type Primitive%20Component%20Object%20Reference) (OtherActor :type Actor%20Object%20Reference) (OtherComp :type Primitive%20Component%20Object%20Reference) (OtherBodyIndex :type Integer) (bFromSweep :type Boolean) (SweepResult :type Hit%20Result%20Structure%20%28by%20ref%29)))

(event EventBeginPlay
  (bind _returnvalue (Math|Random|RandomUnitVector))
  (bind _staticmesh (Variables|Default|GetStaticMesh))
  (bind (_x _y) (Math|Vector|BreakVector _returnvalue))
  (Physics|AddForce _staticmesh (* (Math|Vector|MakeVector _x _y 0.0) (Math|Random|RandomFloatinRange 0.0 1e+01)) "None" false)
  (Utilities|FlowControl|Delay 1.0)
  (Physics|SetSimulatePhysics _staticmesh false))

(event Collision|EventActorBeginOverlap
  (params (OtherActor :type Actor%20Object%20Reference)))

(event EventTick
  (params (DeltaSeconds :type Float%20%28single-precision%29)))

(fn ConstructionScript)

(fn OnPickUp
  (params (InActor :type Actor%20Object%20Reference) (Value :type Integer))
  (if (Actor|ActorHasTag InActor "Player")
    (bind _asgi_custom_game_instance (Utilities|Casting|CastToGI_CustomGameInstance (Game|GetGameInstance))
      (:then
        (Variables|/Game/MyStuff/Blueprints/GI_CustomGameInstance.GI_CustomGameInstance_C|SetScore _asgi_custom_game_instance (+ Value (Variables|/Game/MyStuff/Blueprints/GI_CustomGameInstance.GI_CustomGameInstance_C|GetScore _asgi_custom_game_instance)))
        (Actor|DestroyActor))
      (:CastFailed
        (Development|PrintString "Error" true true "(R=1.000000,G=0.082320,B=0.000000,A=1.000000)")))))