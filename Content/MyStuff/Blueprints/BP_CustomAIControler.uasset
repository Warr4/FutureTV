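; AI controller for BP_TestEnemy that wanders until it spots a pawn tagged "Player", then chases and shoots.
; A looping timer picks random navigable points until PawnSensing latches SeenPlayer and starts a chase timer that re-issues AIMoveTo when the player moves.
; Arriving within range clears that timer through a DoOnce and starts FIRE, which faces the player and spawns BP_DebugProjectile.
; FIRE repeats while the player stays still, otherwise reopens the DoOnce.
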(event OnSeePawn(PawnSensing1)
  (params (Pawn :type Pawn%20Object%20Reference))
  (bind _output_get (Variables|Default|SetPlayer Pawn))
  (if (Actor|ActorHasTag _output_get "Player")
    (Variables|Default|SetSeenPlayer true)
    (bind _returnvalue (Utilities|Time|SetTimerbyEvent (delegate Custom|Move%20to%20player) 0.5 true true))
    (Variables|Default|SetMove%20timer _returnvalue)))

(event Custom|Random%20move
  (if (not (Variables|Default|GetSeenPlayer))
    (bind _randomlocation (Class|NavigationSystemV1|GetRandomLocationinNavigableRadius (Transformation|GetActorLocation (Pawn|GetControlledPawn)) 1e+03 0 0))
    (AI|AIMoveTo 0 _randomlocation 0 5.0 false)))

(event Custom|Open%20Do%20Once
  (Utilities|FlowControl|DoOnce false) ; enters at Reset
)

(event Custom|Move%20to%20player
  (bind _player (Variables|Default|GetPlayer))
  (bind _returnvalue (Transformation|GetActorLocation _player))
  (if (not (Utilities|Operators|EqualEqual (Variables|Default|GetPlayer%20loc) _returnvalue 0.0))
    (Variables|Default|SetPlayer%20loc _returnvalue)
    (AI|AIMoveTo 0 _returnvalue 0 5e+02 false
      (:OnSuccess
        (if (Utilities|IsValid (Variables|Default|GetEnemyRef))
          (Utilities|FlowControl|DoOnce false
            (:Completed
              (Utilities|Time|ClearandInvalidateTimerbyHandle (Variables|Default|GetMove%20timer))
              (CallFunction|FIRE))))))))

(event Custom|FIRE
  (bind _enemyref (Variables|Default|GetEnemyRef))
  (if (Variables|Default|GetCanShoot)
    (Transformation|SetActorRotation _enemyref (Math|Rotator|FindLookatRotation (Transformation|GetActorLocation _enemyref) (Transformation|GetActorLocation (Variables|Default|GetPlayer))))
    (Game|SpawnActorfromClass "/Game/MyStuff/Blueprints/BP_DebugProjectile.BP_DebugProjectile_C" (Variables|/Game/MyStuff/Blueprints/BP_TestEnemy.BP_TestEnemy_C|GetBulletRef _enemyref) "AlwaysSpawn" "MultiplyWithRoot" 0 0)
    (Variables|Default|SetCanShoot false)
    (if (Utilities|Operators|EqualEqual (Variables|Default|GetPlayer%20loc) (Transformation|GetActorLocation (Variables|Default|GetPlayer)) 0.0)
      (Utilities|FlowControl|Delay 1.0)
      (Variables|Default|SetCanShoot true)
      (CallFunction|FIRE)
      (else
        (Utilities|FlowControl|Delay 1.0)
        (Variables|Default|SetCanShoot true)
        (CallFunction|OpenDoOnce)))))

(event EventBeginPlay
  (Utilities|Time|SetTimerbyEvent (delegate Custom|Random%20move) 3.0 true true)
  (bind _asbp_test_enemy (Utilities|Casting|CastToBP_TestEnemy (Pawn|GetControlledPawn)))
  (Variables|Default|SetEnemyRef _asbp_test_enemy))

(event EventTick
  (params (DeltaSeconds :type Float%20%28single-precision%29)))

(fn ConstructionScript)