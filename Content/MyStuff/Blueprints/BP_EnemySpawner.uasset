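; BP_EnemySpawner is a spawner actor that creates a batch of actors of a configurable class when play begins.
; On BeginPlay, a while loop counts Amount down to zero, spawning one SpawningClass instance per pass at the spawner's own transform.
; All spawns happen at once in the same spot, with collision handling left undefined and no delay, offset or respawn logic.
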(event EventBeginPlay
  (while (not (<= (Variables|Default|GetAmount) 0))
    (Variables|Default|SetAmount (+ (Variables|Default|GetAmount) -1))
    (Game|SpawnActorfromClass (Variables|Default|GetSpawningClass) (Transformation|GetActorTransform) "Undefined" "MultiplyWithRoot" 0 0)))

(event Collision|EventActorBeginOverlap
  (params (OtherActor :type Actor%20Object%20Reference)))

(event EventTick
  (params (DeltaSeconds :type Float%20%28single-precision%29)))

(fn ConstructionScript)