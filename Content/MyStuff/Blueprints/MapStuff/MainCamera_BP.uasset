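; MainCamera_BP is a camera actor that makes itself the first player's view target when play begins.
; BeginPlay checks that player controller 0 is valid, then calls SetViewTargetWithBlend on itself.
; An unconnected chain would place the camera a Height offset above the controlled pawn, but it never runs.
; Tick is empty, so the Blueprint has no active follow logic.
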(event EventBeginPlay
  (bind _returnvalue (Game|GetPlayerController 0))
  (Utilities|IsValid _returnvalue
    (:Is%20Valid
      (Game|Player|SetViewTargetwithBlend _returnvalue self 0.0 "VTBlend_Linear" 0.0 false))))

(event EventTick
  (params (DeltaSeconds :type Float%20%28single-precision%29)))

(fn ConstructionScript)