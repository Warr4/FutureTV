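; BP_CameraMover is a trigger volume that advances the main camera when the player enters it with no enemy bots left.
; On Box overlap by an actor tagged Player, it checks that no BP_BotTest actors exist in the level.
; It then sets MainCamera's TargetLoc to the location of its WaveControler reference and calls MoveCamera.
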(event OnComponentBeginOverlap(Box)
  (params (OverlappedComponent :type Primitive%20Component%20Object%20Reference) (OtherActor :type Actor%20Object%20Reference) (OtherComp :type Primitive%20Component%20Object%20Reference) (OtherBodyIndex :type Integer) (bFromSweep :type Boolean) (SweepResult :type Hit%20Result%20Structure%20%28by%20ref%29))
  (bind _maincamera (Variables|Default|GetMainCamera))
  (if (Actor|ActorHasTag OtherActor "Player")
    (bind _outactors (Actor|GetAllActorsOfClass "/Game/MyStuff/Blueprints/AiStuff/BP_BotTest.BP_BotTest_C"))
    (if (== (Utilities|Array|Length _outactors) 0)
      (Variables|/Game/MyStuff/Blueprints/MapStuff/MainCamera_BP.MainCamera_BP_C|SetTargetLoc _maincamera (Transformation|GetActorLocation (Variables|Default|GetWaveControler)))
      (Default|MoveCamera _maincamera))))

(event EventBeginPlay)

(event Collision|EventActorBeginOverlap
  (params (OtherActor :type Actor%20Object%20Reference)))

(event EventTick
  (params (DeltaSeconds :type Float%20%28single-precision%29)))

(fn ConstructionScript)