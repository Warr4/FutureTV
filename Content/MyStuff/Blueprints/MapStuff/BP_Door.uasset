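; Door Blueprint that drops its cube out of the way when a qualifying actor enters its trigger box, then restores it on a timer.
; Overlap opens it for actors tagged PlayerDamageable, or Player while the custom GameInstance reports respawning.
; Each overlap schedules Close, with a FlipFlop clearing the stored timer on alternate entries.
; Movement is an instant teleport relative to the location cached at BeginPlay.
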(event OnComponentBeginOverlap(Box)
  (params (OverlappedComponent :type Primitive%20Component%20Object%20Reference) (OtherActor :type Actor%20Object%20Reference) (OtherComp :type Primitive%20Component%20Object%20Reference) (OtherBodyIndex :type Integer) (bFromSweep :type Boolean) (SweepResult :type Hit%20Result%20Structure%20%28by%20ref%29))
  (Utilities|FlowControl|FlipFlop
    (:A
      _)
    (:B
      (Utilities|Time|ClearandInvalidateTimerbyHandle (Variables|Default|GetNewVar))))
  (bind _returnvalue (Utilities|Time|SetTimerbyEvent (delegate Custom|Close) 2.0))
  (Variables|Default|SetNewVar _returnvalue)
  (Utilities|FlowControl|Sequence
    (:then_0
      (if (Actor|ActorHasTag OtherActor "PlayerDamageable")
        (CallFunction|Open :!label _label)))
    (:then_1
      (if (Variables|/Game/MyStuff/Blueprints/GI_CustomGameInstance.GI_CustomGameInstance_C|GetIsRespawning (Variables|Default|GetGame%20Instance))
        (if (Actor|ActorHasTag OtherActor "Player")
          (goto _label))))))

(event OnComponentEndOverlap(Box)
  (params (OverlappedComponent :type Primitive%20Component%20Object%20Reference) (OtherActor :type Actor%20Object%20Reference) (OtherComp :type Primitive%20Component%20Object%20Reference) (OtherBodyIndex :type Integer)))

(event Custom|Close
  (Transformation|SetRelativeLocation (Variables|Default|GetCube) (Variables|Default|GetCloseValue) false true))

(event Custom|Open
  (bind _closevalue (Variables|Default|GetCloseValue))
  (Transformation|SetRelativeLocation (Variables|Default|GetCube) (Math|Vector|MakeVector (.x _closevalue) (.y _closevalue) (+ (.z _closevalue) -2e+02)) false true))

(event EventBeginPlay
  (bind _asgi_custom_game_instance (Utilities|Casting|CastToGI_CustomGameInstance (Game|GetGameInstance)))
  (Variables|Default|SetGame%20Instance _asgi_custom_game_instance)
  (Variables|Default|SetCloseValue (Variables|/Script/Engine.SceneComponent|GetRelativeLocation (Variables|Default|GetCube))))

(event Collision|EventActorBeginOverlap
  (params (OtherActor :type Actor%20Object%20Reference)))

(fn ConstructionScript)