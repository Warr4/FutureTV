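; BP_WaveControler runs an enemy wave encounter that opens a linked door after the final wave.
; The first Player-tagged actor to overlap its Box starts a looping one-second timer that counts living actors of EnemyType.
; When none remain, it advances CurrentWave, looks up the spawn amount in the Waves map (five hardcoded cases) and triggers every controlled spawner.
; Once CurrentWave exceeds MaxWave, it opens OpeningDoor once; the timer is never cleared.
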(event OnComponentBeginOverlap(Box)
  (params (OverlappedComponent :type Primitive%20Component%20Object%20Reference) (OtherActor :type Actor%20Object%20Reference) (OtherComp :type Primitive%20Component%20Object%20Reference) (OtherBodyIndex :type Integer) (bFromSweep :type Boolean) (SweepResult :type Hit%20Result%20Structure%20%28by%20ref%29))
  (if (Actor|ActorHasTag OtherActor "Player")
    (Utilities|FlowControl|DoOnce false
      (:Completed
        (Utilities|Time|SetTimerbyEvent (delegate Custom|HowManyShitsExists) 1.0 true)))))

(event Custom|HowManyShitsExists
  (bind _outactors (Actor|GetAllActorsOfClass (Variables|Default|GetEnemyType)))
  (if (== (Utilities|Array|Length _outactors) 0)
    (bind _output_get (Variables|Default|SetCurrentWave (+ (Variables|Default|GetCurrentWave) 1)))
    (if (> _output_get (Variables|Default|GetMaxWave))
      (Development|PrintString "Wave Complete")
      (Utilities|FlowControl|DoOnce false
        (:Completed
          (Default|Open (Variables|Default|GetOpeningDoor))))
      (else
        (switch int (Variables|Default|GetCurrentWave)
          (:1
            (Variables|Default|SetEnemySpawnAmount (.Value (Utilities|Map|Find (Variables|Default|GetWaves) "Wave1"))))
          (:2
            (Variables|Default|SetEnemySpawnAmount (.Value (Utilities|Map|Find (Variables|Default|GetWaves) "Wave2"))))
          (:3
            (Variables|Default|SetEnemySpawnAmount (.Value (Utilities|Map|Find (Variables|Default|GetWaves) "Wave3"))))
          (:4
            (Variables|Default|SetEnemySpawnAmount (.Value (Utilities|Map|Find (Variables|Default|GetWaves) "Wave4"))))
          (:5
            (Variables|Default|SetEnemySpawnAmount (.Value (Utilities|Map|Find (Variables|Default|GetWaves) "Wave5")))))
        (CallFunction|StartWave)))
    (else
      (Development|PrintString (Utilities|String|ToString(Integer) (Utilities|Array|Length _outactors)) true true "(R=1.000000,G=0.000000,B=0.000000,A=1.000000)" 1.0))))

(event Custom|StartWave
  (for _array_element (Variables|Default|GetControled%20Spawners)
    (Variables|/Game/MyStuff/Blueprints/BP_EnemySpawner.BP_EnemySpawner_C|SetAmount _array_element (Variables|Default|GetEnemySpawnAmount))
    (Default|Spawn _array_element)))

(event Collision|EventActorBeginOverlap
  (params (OtherActor :type Actor%20Object%20Reference)))

(event EventTick
  (params (DeltaSeconds :type Float%20%28single-precision%29)))

(fn ConstructionScript)