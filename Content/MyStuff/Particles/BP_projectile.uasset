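; BP_projectile is a projectile Blueprint whose only graph logic sizes its component R when play begins.
; BeginPlay keeps R's relative location and rotation and multiplies its existing scale, divided by 100, by Radius on X and Y and by Length on Z.
; The construction script is empty, and the graphs contain no movement or collision logic.
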(event EventBeginPlay
  (bind _r (Variables|Default|Getr))
  (bind _returnvalue (Transformation|GetRelativeTransform _r))
  (Transformation|SetRelativeTransform _r (Math|Transform|MakeTransform (.location _returnvalue) (.rotation _returnvalue) (Math|Vector|MakeVector (* (/ (.x (.scale _returnvalue)) 1e+02) (Variables|Default|GetRadius)) (* (/ (.y (.scale _returnvalue)) 1e+02) (Variables|Default|GetRadius)) (* (/ (.z (.scale _returnvalue)) 1e+02) (Variables|Default|GetLength)))) false false))

(fn ConstructionScript)